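; Player character Blueprint that handles movement, turning and death, handing off to the next player when the viewed character dies.
; Adds the Enhanced Input mapping context for local controllers, driving actor-relative movement and controller yaw and pitch.
; Health component death plays a sound, hides the mesh and spawns an explosion.
; Outside dedicated servers, a second death handler, bound only while view target, calls PossessNextPlayer on player controller 0.
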(event `self.ReceiveControllerChanged`
  (params (OldController :type "Controller Object Reference") (NewController :type "Controller Object Reference"))
  (bind _asplayer_controller (cast `PlayerController` NewController))
  (if (`Controller.IsLocalPlayerController` _asplayer_controller)
    (`EnhancedInputSubsystemInterface.AddMappingContext` (pcsubsystem `EnhancedInputLocalPlayerSubsystem` _asplayer_controller) "/Game/Characters/IMC_Character.IMC_Character" 0 (struct))))

(event `EnhancedInput|/Game/Characters/InputAction_Move`
  (params (ActionValue :type "Vector2D Structure") (ElapsedSeconds :type "Float (double-precision)") (TriggeredSeconds :type "Float (double-precision)") (InputAction :type "InputAction Object Reference" :default "/Game/Characters/InputAction_Move.InputAction_Move"))
  (bind _returnvalue (`self.K2_GetActorRotation`))
  (:`Triggered`
    (`self.AddMovementInput` (`KismetMathLibrary.GetRightVector` _returnvalue) ActionValue_X)
    (`self.AddMovementInput` (`KismetMathLibrary.GetForwardVector` _returnvalue) ActionValue_Y)))

(event `EnhancedInput|/Game/Characters/InputAction_Turn`
  (params (ActionValue :type "Vector2D Structure") (ElapsedSeconds :type "Float (double-precision)") (TriggeredSeconds :type "Float (double-precision)") (InputAction :type "InputAction Object Reference" :default "/Game/Characters/InputAction_Turn.InputAction_Turn"))
  (:`Triggered`
    (`self.AddControllerYawInput` ActionValue_X)
    (`self.AddControllerPitchInput` ActionValue_Y)))

(event `self.Health.Died`
  (params (DiedActor :type "Actor Object Reference"))
  (bind _returnvalue (`self.K2_GetActorLocation`))
  (`GameplayStatics.PlaySoundAtLocation` "/Engine/EditorSounds/Notifications/CompileFailed.CompileFailed" _returnvalue (struct) 1.0 1.0 0.0 null null null null)
  (`SceneComponent.SetHiddenInGame` (`self.Mesh`) true false)
  (`NiagaraFunctionLibrary.SpawnSystemAtLocation` "/Niagara/DefaultAssets/Templates/Systems/SimpleExplosion.SimpleExplosion" _returnvalue))

(event `self.K2_OnBecomeViewTarget`
  (params (PC :type "PlayerController Object Reference"))
  (if (not (`KismetSystemLibrary.IsDedicatedServer`))
    (add `HealthComponent.Died` (`self.Health`) (delegate `Died_Event`))))

(event `Died_Event`
  (params (DiedActor :type "Actor Object Reference"))
  (bind _asbp_player_controller (cast `/Game/Modes/SquidGame/BP_PlayerController` (`GameplayStatics.GetPlayerControllerFromID` 0)))
  (`/Game/Modes/SquidGame/BP_PlayerController.PossessNextPlayer` _asbp_player_controller))

(event `self.K2_OnEndViewTarget`
  (params (PC :type "PlayerController Object Reference"))
  (if (not (`KismetSystemLibrary.IsDedicatedServer`))
    (remove `HealthComponent.Died` (`self.Health`) (delegate `Died_Event`))))

(fn `UserConstructionScript`)