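; Player controller for the Squid Game mode that lets a dead player spectate surviving players.
; On BeginPlay it adds an input mapping context for the local controller; its possess-next input acts only when the controlled character is dead.
; PossessNextPlayer collects living characters from the game state's PlayerArray, drops the current view target and blends the camera to a random pick.
; Despite the name, it changes only the view target, never possession.
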(event `self.ReceiveBeginPlay`
  (if (`self.IsLocalPlayerController`)
    (`EnhancedInputSubsystemInterface.AddMappingContext` (subsystem `EnhancedInputLocalPlayerSubsystem`) "/Game/Modes/SquidGame/IMC_Possion.IMC_Possion" 0 (struct))))

(event `EnhancedInput|/Game/Modes/SquidGame/InputAction_PossessNextPlayer`
  (params (ActionValue :type Boolean) (ElapsedSeconds :type "Float (double-precision)") (TriggeredSeconds :type "Float (double-precision)") (InputAction :type "InputAction Object Reference" :default "/Game/Modes/SquidGame/InputAction_PossessNextPlayer.InputAction_PossessNextPlayer"))
  (:`Started`
    (bind _asbp_character (cast `/Game/Characters/BP_Character` (`self.K2_GetPawn`)))
    (if (`HealthComponent.IsDead` (`/Game/Characters/BP_Character.Health` _asbp_character))
      (`self.PossessNextPlayer`))))

(fn `PossessNextPlayer`
  (locals (Characters :type "Array of /Game/Characters/BP_Character Object Reference"))
  (bind _characters (`local.Characters`))
  (bind _output (`|GetArrayItem` _characters (`KismetMathLibrary.RandomIntegerInRange` 0 (- (`KismetArrayLibrary.Array_Length` _characters) 1))))
  (bind _assquid_game_state (cast `SquidGameState` (`GameplayStatics.GetGameState`)))
  (for _array_element (`GameStateBase.PlayerArray` _assquid_game_state)
    (bind _assquid_player_state (cast `SquidPlayerState` _array_element))
    (if (not (`SquidPlayerState.IsDead` _assquid_player_state))
      (bind _asbp_character (cast `/Game/Characters/BP_Character` (`PlayerState.GetPawn` _assquid_player_state)))
      (`KismetArrayLibrary.Array_Add` (`local.Characters`) _asbp_character)))
  (`|ExecutionSequence`
    (:`then_0`
      (bind _asbp_character_2 (cast `/Game/Characters/BP_Character` (`self.GetViewTarget`)))
      (`KismetArrayLibrary.Array_RemoveItem` (`local.Characters`) _asbp_character_2))
    (:`then_1`
      (`/Engine/EditorBlueprintResources/StandardMacros.IsValid` _output
        (:`Is Valid`
          (`self.SetViewTargetWithBlend` _output 0.0 "VTBlend_EaseIn"))))))

(fn `UserConstructionScript`)