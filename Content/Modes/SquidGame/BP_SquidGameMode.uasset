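; Game mode for a Squid Game red light, green light round with a doll watcher.
; On match start it sets the game state's timer, starts behavior tree logic after a delay, and kills unfinished players when time expires.
; When the doll finishes turning to watch, player transforms are saved.
; Tick then kills unfinished players who deviate beyond a small tolerance, via their HealthComponent and a forced net update.
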(event `self.MatchHasStarted`
  (bind _startdelayafterallplayersconnected (`self.StartDelayAfterAllPlayersConnected`))
  (bind _assquid_game_state (cast `SquidGameState` (`GameplayStatics.GetGameState`)))
  (`SquidGameState.SetGameDuration` _assquid_game_state _startdelayafterallplayersconnected (`self.GameDuration`))
  (`KismetSystemLibrary.Delay` _startdelayafterallplayersconnected)
  (`BrainComponent.StartLogic` (`self.BehaviorTree`))
  (`KismetSystemLibrary.Delay` (`self.GameDuration`))
  (bind _playerstate (`self.ForEachPlayer`)
    (:`Out`
      (`self.KillPlayerIfPossible` _playerstate))))

(event `self.ReceiveBeginPlay`
  (bind _returnvalue (`GameplayStatics.GetActorOfClass` "/Game/Doll/BP_Doll.BP_Doll_C"))
  (bind _output_get (set `self.Doll` _returnvalue))
  (`/Engine/EditorBlueprintResources/StandardMacros.IsValid` _output_get
    (:`Is Valid`
      (add `/Game/Doll/BP_Doll.FinishedRotationAndWatching` _output_get (delegate `FinishedRotationAndWatching_Event`)))))

(event `FinishedRotationAndWatching_Event`
  (bind _playerstate (`self.ForEachPlayer`)
    (:`Out`
      (`SquidPlayerState.RememberTransform` _playerstate))))

(event `self.ReceiveTick`
  (params (DeltaSeconds :type "Float (single-precision)"))
  (bind _doll (`self.Doll`)
    (:`then`
      (if (`/Game/Doll/BP_Doll.IsWatchingAndRotationLastTick` _doll)
        (bind _playerstate (`self.ForEachPlayer`)
          (:`Out`
            (if (not (`SquidPlayerState.IsFinishLineCrossed` _playerstate))
              (bind _returnvalue (`PlayerState.GetPawn` _playerstate))
              (`/Engine/EditorBlueprintResources/StandardMacros.IsValid` _returnvalue
                (:`Is Valid`
                  (bind (_returnvalue_location _returnvalue_rotation) (`KismetMathLibrary.BreakTransform` (`self.GetTransform` _returnvalue)))
                  (bind (_returnvalue_location_2 _returnvalue_rotation_2) (`KismetMathLibrary.BreakTransform` (`SquidPlayerState.GetLastAllowedToMoveTransform` _playerstate)))
                  (if (not (and (== _returnvalue_location _returnvalue_location_2 :`ErrorTolerance` 1.0) (== _returnvalue_rotation _returnvalue_rotation_2 :`ErrorTolerance` 0.1)))
                    (`self.KillPlayerIfPossible` _playerstate)))))))))
    (:`else`)))

(fn `KillPlayerIfPossible`
  (params (PlayerState :type "SquidPlayerState Object Reference"))
  (bind _returnvalue (`PlayerState.GetPawn` PlayerState))
  (bind _returnvalue_2 (`self.GetComponentByClass` _returnvalue "/Script/Game.HealthComponent"))
  (if (not (`SquidPlayerState.IsFinishLineCrossed` PlayerState))
    (`/Engine/EditorBlueprintResources/StandardMacros.IsValid` _returnvalue
      (:`Is Valid`
        (`/Engine/EditorBlueprintResources/StandardMacros.IsValid` _returnvalue_2
          (:`Is Valid`
            (`HealthComponent.Die` _returnvalue_2)
            (`self.ForceNetUpdate` _returnvalue)))))))

(fn `UserConstructionScript`)