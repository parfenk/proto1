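; BP_SafeZone is a finish-line trigger that assigns placements to players who reach it in a Squid game mode.
; On overlap, only the server acts, and only for pawns with a SquidPlayerState that has not yet crossed the finish line.
; It sets that player's place to one above the game state's crossed-player count, then forces a net update of the player state.
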(event `self.ReceiveActorBeginOverlap`
  (params (OtherActor :type "Actor Object Reference"))
  (`/Engine/EditorBlueprintResources/ActorMacros.Switch Has Authority`
    (:`Authority`
      (bind _aspawn (cast `Pawn` OtherActor))
      (bind _assquid_player_state (cast `SquidPlayerState` (`Pawn.PlayerState` _aspawn)))
      (if (not (`SquidPlayerState.IsFinishLineCrossed` _assquid_player_state))
        (bind _assquid_game_state (cast `SquidGameState` (`GameplayStatics.GetGameState`)))
        (`SquidPlayerState.SetPlace` _assquid_player_state (+ (`SquidGameState.GetNumPlayersCrossedFinishLine` _assquid_game_state) 1))
        (`self.ForceNetUpdate` _assquid_player_state)))))

(fn `UserConstructionScript`)