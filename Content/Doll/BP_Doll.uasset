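; BP_Doll is a doll actor that turns between a watching pose and a resting pose, half a turn apart, based on its watching state.
; Each tick it rotates at a constant speed toward the pose for that state, and a click sound plays whenever the state changes.
; A last-tick flag edge-detects when it is both watching and fully turned, firing the finished-rotation-and-watching call once per turn.
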(event `self.ReceiveBeginPlay`
  (add `self.WatchingStateChanged` (delegate `WatchingStateChanged_Event`)))

(event `WatchingStateChanged_Event` :!signature `self.WatchingStateChanged`
  (params (bNewWatching :type Boolean))
  (`GameplayStatics.PlaySoundAtLocation` "/Engine/VREditor/Sounds/UI/Click_on_Button_Cue.Click_on_Button_Cue" (`self.K2_GetActorLocation`) (struct) 1.0 1.0 0.0 null null null null))

(event `self.ReceiveTick`
  (params (DeltaSeconds :type "Float (single-precision)"))
  (`self.K2_SetActorRotation` (`KismetMathLibrary.RInterpTo_Constant` (`self.K2_GetActorRotation`) (`self.GetDesiredRotation`) DeltaSeconds (`self.GetRotationSpeed`)))
  (`self.UpdateIsWatchingAndRotated`))

(fn `GetDesiredRotation`
  (returns (ReturnValue :type "Rotator Structure"))
  (return (`KismetMathLibrary.SelectRotator` (struct :`Yaw` 180.0) (struct) (`self.IsWatching`))))

(fn `UpdateIsWatchingAndRotated`
  (locals (IsWatchingAndRotation :type Boolean))
  (set `local.IsWatchingAndRotation` (and (`self.IsWatching`) (== (`self.K2_GetActorRotation`) (`self.GetDesiredRotation`) :`ErrorTolerance` 0.1)))
  (`|ExecutionSequence`
    (:`then_0`
      (if (and (not (`self.IsWatchingAndRotationLastTick`)) (`local.IsWatchingAndRotation`))
        (`self.FinishedRotationAndWatching`)))
    (:`then_1`
      (set `self.IsWatchingAndRotationLastTick` (`local.IsWatchingAndRotation`)))))

(fn `UserConstructionScript`)